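; BP_Player is the player character, with movement, jumping, hold-Shift sprint and a spotlight toggled on F.
; E fires a short camera line trace that either increments a BP_Switch's metallic-door count or stores and hides a BP_Key in Inventory.
; BeginPlay creates the inventory widget and passes it the player reference, while Tick sets walk speed from the Run flag.
; The Box overlap with Door_01 checks the first inventory slot but takes no action.
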(event `self.ReceiveBeginPlay`
  (bind _returnvalue (`|CreateWidget` "/Game/UI/Inventory_Widget.Inventory_Widget_C"))
  (`UserWidget.AddToViewport` _returnvalue 0)
  (set `/Game/UI/Inventory_Widget.Player` self _returnvalue))

(event `Key|E`
  (params (Key :type "Key Structure"))
  (bind _camera (`self.Camera`))
  (bind _returnvalue (`SceneComponent.K2_GetComponentLocation` _camera))
  (:`Pressed`
    (bind (_outhit _returnvalue_2) (`KismetSystemLibrary.LineTraceSingleForObjects` :`Start` _returnvalue :`End` (+ _returnvalue (* (`SceneComponent.GetForwardVector` _camera) 300.0)) :`ObjectTypes` (`|MakeArray` "ObjectTypeQuery1" :!type "EObjectTypeQuery Enum") :`DrawDebugType` "ForDuration"))
    (if _returnvalue_2
      (bind (_bblockinghit _binitialoverlap _time _distance _location _impactpoint _normal _impactnormal _physmat _hitactor) (`GameplayStatics.BreakHitResult` _outhit))
      (bind _asbp_switch (cast `/Game/Assets/SomeFBX/BP_Switch` _hitactor)
        (:`then`
          (`/Game/Assets/SomeFBX/BP_Switch.Added Count For Metallic Door` _asbp_switch))
        (:`CastFailed`
          (bind _asbp_key (cast `/Game/Scripts/BP_Key` _hitactor))
          (`KismetArrayLibrary.Array_Set` (`self.Inventory`) 0 _asbp_key)
          (`self.SetActorHiddenInGame` _asbp_key true))))))

(event `self.ReceiveTick`
  (params (DeltaSeconds :type "Float (single-precision)"))
  (bind _charactermovement (`self.CharacterMovement`))
  (if (`self.Run`)
    (set `CharacterMovementComponent.MaxWalkSpeed` 800.0 _charactermovement)
    (else
      (set `CharacterMovementComponent.MaxWalkSpeed` 500.0 _charactermovement))))

(event `InputAxis|MoveForward`
  (params (AxisValue :type "Float (single-precision)"))
  (`self.AddMovementInput` (`self.GetActorForwardVector`) AxisValue))

(event `InputAxis|LookHorizontal`
  (params (AxisValue :type "Float (single-precision)"))
  (`self.AddControllerYawInput` AxisValue))

(event `InputAxis|LookVertical`
  (params (AxisValue :type "Float (single-precision)"))
  (`self.AddControllerPitchInput` AxisValue))

(event `InputAxis|MoveRight`
  (params (AxisValue :type "Float (single-precision)"))
  (`self.AddMovementInput` (`self.GetActorRightVector`) AxisValue))

(event `InputAction|Jump`
  (params (Key :type "Key Structure"))
  (:`Pressed`
    (`self.Jump`)))

(event `Key|F`
  (params (Key :type "Key Structure"))
  (:`Pressed`
    (bind _output_get (set `self.VisibilityLight` (not (`self.VisibilityLight`))))
    (`SceneComponent.SetVisibility` (`self.SpotLight`) _output_get false)))

(event `Key|LeftShift`
  (params (Key :type "Key Structure"))
  (:`Pressed`
    (set `self.Run` (not (`self.Run`)) :!label _label))
  (:`Released`
    (goto _label)))

(event `self.Box.OnComponentBeginOverlap`
  (params (OverlappedComponent :type "PrimitiveComponent Object Reference") (OtherActor :type "Actor Object Reference") (OtherComp :type "PrimitiveComponent Object Reference") (OtherBodyIndex :type Integer) (bFromSweep :type Boolean) (SweepResult :type "HitResult Structure (by ref)"))
  (cast `/Game/Assets/MultistoryDungeons/Blueprints/Doors/Door_01` OtherActor)
  (if (== (`|GetArrayItem` (`self.Inventory`)) null)
    _))

(fn `UserConstructionScript`
  (`SceneComponent.SetVisibility` (`self.SpotLight`) (`self.VisibilityLight`) false))