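; AI controller for BP_Enemy that patrols random TargetPoints and reacts to sight and noise.
; Perception updates chase the sensed actor, or move to the last stimulus location and resume patrol after a delay.
; Tick infers movement from position changes, triggering a new patrol move when idle and not hunting.
; HearNoise investigates player noises before resuming, though its range check measures the player against itself.
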(event `self.ReceiveBeginPlay`
  ;[1 1 1] Начало
  (bind _asbp_enemy (cast `/Game/Scripts/Blueprints/NPC/BP_Enemy` (`self.K2_GetPawn`)))
  (bind _output_get (set `self.AICharacter` _asbp_enemy))
  (set `self.PrevPos` (`self.K2_GetActorLocation` _output_get))
  (`self.MoveOnRoute`))

(event `self.AIPerception.OnTargetPerceptionUpdated`
  (params (Actor :type "Actor Object Reference") (Stimulus :type "AIStimulus Structure"))
  (bind (_age _expirationage _strength _stimuluslocation _receiverlocation _tag _bsuccessfullysensed) (break `AIStimulus` Stimulus))
  ;[1 1 1] При вхождении в зону видимости начинает преследдование. Если уходит из зоны видимости, то идет в последнюю точку, где видел его. После этого ждет 3 секунды. И продолжает патрулирование
  (if _bsuccessfullysensed
    (`self.StopMovement`)
    (set `self.IsAtManhaunt` true)
    (`self.MoveToActor` Actor -1.0 true true true null)
    (else
      (`self.StopMovement`)
      (`self.MoveToLocation` _stimuluslocation -1.0 true true false true null)
      (`KismetSystemLibrary.Delay` 8.0)
      (set `self.IsAtManhaunt` false)
      (`self.MoveOnRoute`))))

(event `self.ReceiveTick`
  (params (DeltaSeconds :type "Float (single-precision)"))
  ;[1 1 1] Проверка на нахождении пешки в движении.
  (set `self.CurPos` (`self.K2_GetActorLocation` (`self.AICharacter`)))
  (if (== (`KismetMathLibrary.Conv_VectorToQuaternion` (`self.PrevPos`)) (`KismetMathLibrary.Conv_VectorToQuaternion` (`self.CurPos`)) 1e-05)
    (set `self.IsAtMove` false)
    (else
      (set `self.IsAtMove` true)))
  (set `self.PrevPos` (`self.K2_GetActorLocation` (`self.AICharacter`)))
  (if (not (`self.IsAtManhaunt`))
    (`self.MoveOnRoute`)))

(event `HearNoise`
  (params (LocationOfNoise :type "Vector Structure") (SourceOfNoise :type "Actor Object Reference"))
  ;[1 1 1] Проверка на шум
  (set `self.IsAtManhaunt` true)
  (bind _asbp_player (cast `/Game/Scripts/Blueprints/Player/BP_Player` SourceOfNoise))
  (if (<= (`self.GetDistanceTo` _asbp_player SourceOfNoise) (`self.PlayerHearingDistance`))
    (`self.MoveToLocation` LocationOfNoise -1.0 true true false true null)
    (`KismetSystemLibrary.Delay` 15.0)
    (set `self.IsAtManhaunt` false)
    (`self.MoveOnRoute`)))

(fn `MoveOnRoute`
  (if (not (`self.IsAtMove`))
    (bind _outactors (`GameplayStatics.GetAllActorsOfClass` "/Script/Engine.TargetPoint"))
    (`self.MoveToActor` (`|GetArrayItem` _outactors (`KismetMathLibrary.RandomIntegerInRange` 0 (`KismetArrayLibrary.Array_LastIndex` _outactors))) -1.0 true true true null)))

(fn `UserConstructionScript`)