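; First-person player character for level 2, with walk and jump movement, Shift sprinting and an F-key flashlight toggle.
; While move speed equals run speed, Tick reports the player's location to the Monster through HearNoise and prints it.
; E line-traces from the camera: switches add to the metallic door count, and a bronze door with true Status loads the Minimal_Default level.
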(event `self.ReceiveTick`
  (params (DeltaSeconds :type "Float (single-precision)"))
  (bind _returnvalue (`self.K2_GetActorLocation` self))
  (if (== (`CharacterMovementComponent.MaxWalkSpeed` (`self.CharacterMovement`)) (`self.RunSpeed`))
    (`/Game/Scripts/Blueprints/NPC/EnemyAI.HearNoise` (`self.Monster`) _returnvalue 3000.0)
    (`KismetSystemLibrary.PrintString` (`KismetStringLibrary.Conv_VectorToString` _returnvalue))))

(event `Key|E`
  (params (Key :type "Key Structure"))
  (bind _camera (`self.Camera`))
  (bind _returnvalue (`SceneComponent.K2_GetComponentLocation` _camera))
  (:`Pressed`
    (bind (_outhit _returnvalue_2) (`KismetSystemLibrary.LineTraceSingleForObjects` :`Start` _returnvalue :`End` (+ _returnvalue (* (`SceneComponent.GetForwardVector` _camera) 300.0)) :`ObjectTypes` (`|MakeArray` "ObjectTypeQuery1" :!type "EObjectTypeQuery Enum") :`DrawDebugType` "ForDuration"))
    (if _returnvalue_2
      (bind (_bblockinghit _binitialoverlap _time _distance _location _impactpoint _normal _impactnormal _physmat _hitactor) (`GameplayStatics.BreakHitResult` _outhit))
      (bind _asbp_switch_for_lvl_2 (cast `/Game/Assets/SomeFBX/BP_Switch_for_lvl2` _hitactor)
        (:`then`
          (`/Game/Assets/SomeFBX/BP_Switch_for_lvl2.Added Count For Metallic Door` _asbp_switch_for_lvl_2))
        (:`CastFailed`
          (bind _asbp_fp_door_bronze_01 (cast `/Game/Assets/MultistoryDungeons/Blueprints/FIRST-PERSON_V2/FP_DoorsAndBars/BP_FP_Door_Bronze_01` _hitactor))
          (if (`/Game/Assets/MultistoryDungeons/Blueprints/FIRST-PERSON_V2/FP_DoorsAndBars/BP_FP_Door_Bronze_01.Status` _asbp_fp_door_bronze_01)
            (`GameplayStatics.OpenLevel` "Minimal_Default")))))))

(event `self.ReceiveBeginPlay`
  (set `CharacterMovementComponent.MaxWalkSpeed` (`self.WalkSpeed`) (`self.CharacterMovement`)))

(event `InputAxis|MoveForward`
  (params (AxisValue :type "Float (single-precision)"))
  (`self.AddMovementInput` (`self.GetActorForwardVector`) AxisValue))

(event `InputAxis|LookHorizontal`
  (params (AxisValue :type "Float (single-precision)"))
  (`self.AddControllerYawInput` AxisValue))

(event `InputAxis|LookVertical`
  (params (AxisValue :type "Float (single-precision)"))
  (`self.AddControllerPitchInput` AxisValue))

(event `InputAxis|MoveRight`
  (params (AxisValue :type "Float (single-precision)"))
  (`self.AddMovementInput` (`self.GetActorRightVector`) AxisValue))

(event `InputAction|Jump`
  (params (Key :type "Key Structure"))
  (:`Pressed`
    (`self.Jump`)))

(event `Key|F`
  (params (Key :type "Key Structure"))
  (:`Pressed`
    (bind _output_get (set `self.VisibilityLight` (not (`self.VisibilityLight`))))
    (`SceneComponent.SetVisibility` (`self.SpotLight`) _output_get false)))

(event `Key|LeftShift`
  (params (Key :type "Key Structure"))
  (bind _charactermovement (`self.CharacterMovement`))
  (:`Pressed`
    (set `CharacterMovementComponent.MaxWalkSpeed` (`self.RunSpeed`) _charactermovement))
  (:`Released`
    (set `CharacterMovementComponent.MaxWalkSpeed` (`self.WalkSpeed`) _charactermovement)))

(fn `UserConstructionScript`
  (`SceneComponent.SetVisibility` (`self.SpotLight`) (`self.VisibilityLight`) false))